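; Player controller for Cardit that drives the controlled character and handles online session hosting and joining.
; Each tick it caches the possessed pawn as the current character and passes it to the in-game HUD widget created on BeginPlay.
; Look, move, jump and fire inputs act on that cached character, with mouse look scaled by sensitivity.
; Debug keys O and P find and join the first session or create one, printing the result.
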(event `Key|O`
  (params (Key :type "Key Structure" :default "AnyKey"))
  (:`Pressed`
    (bind _results (`FindSessionsCallbackProxy.FindSessions` self 10)
      (:`OnSuccess`
        (`KismetSystemLibrary.PrintString` (`KismetStringLibrary.Concat_StrStr` "Found " (`KismetStringLibrary.Conv_IntToString` (`KismetArrayLibrary.Array_Length` _results)) " servers"))
        (`JoinSessionCallbackProxy.JoinSession` self (`KismetArrayLibrary.Array_Get` _results)))
      (:`OnFailure`
        (`KismetSystemLibrary.PrintString` "Find failed")))))

(event `Key|P`
  (params (Key :type "Key Structure" :default "AnyKey"))
  (:`Pressed`
    (`CreateSessionCallbackProxy.CreateSession` self 10
      (:`OnSuccess`
        (`KismetSystemLibrary.PrintString` "Creation successful"))
      (:`OnFailure`
        (`KismetSystemLibrary.PrintString` "Creation failed")))))

(event `self.ReceiveTick`
  (params (DeltaSeconds :type "Float (single-precision)"))
  ;[1 1 1] Get current controlled pawn every tick
  (bind _ascardit_character_bp (cast `/Game/BP/CarditCharacter_BP` (`self.K2_GetPawn`))
    (:`then`
      (bind _output_get (set `self.CurrentCharacter` _ascardit_character_bp))
      (if (`KismetSystemLibrary.IsValid` (`self.CurrentIngameUI`))
        (set `/Game/UI/IngameUI.Character` _output_get (`self.CurrentIngameUI`))))
    (:`CastFailed`
      (set `self.CurrentCharacter` null))))

(event `InputAxis|Turn`
  (params (AxisValue :type "Float (single-precision)"))
  (bind _currentcharacter (`self.CurrentCharacter`))
  ;[1 1 1] Mouse input binding
  (if (`KismetSystemLibrary.IsValid` _currentcharacter)
    (`Pawn.AddControllerYawInput` _currentcharacter (* (/ AxisValue (`self.Sensitivity Constant`)) (`self.Sensitivity`)))))

(event `InputAxis|LookUp`
  (params (AxisValue :type "Float (single-precision)"))
  (bind _currentcharacter (`self.CurrentCharacter`))
  ;[1 1 1] Mouse input binding
  (if (`KismetSystemLibrary.IsValid` _currentcharacter)
    (`Pawn.AddControllerPitchInput` _currentcharacter (* (`self.Sensitivity`) (/ AxisValue (`self.Sensitivity Constant`))))))

(event `InputAction|Fire`
  (params (Key :type "Key Structure" :default "AnyKey"))
  ;[1 1 1] Mouse input binding
  (:`Pressed`
    (if (`KismetSystemLibrary.IsValid` (`self.CurrentCharacter`))
      (`self.FireCurrentWeapon`))))

(event `InputAction|Jump`
  (params (Key :type "Key Structure" :default "AnyKey"))
  (bind _currentcharacter (`self.CurrentCharacter`))
  (bind _returnvalue (`KismetSystemLibrary.IsValid` _currentcharacter))
  ;[1 1 1] Movement binding
  (:`Pressed`
    (if _returnvalue
      (`CarditCharacter.CharStartJumping` _currentcharacter)))
  (:`Released`
    (if _returnvalue
      (`CarditCharacter.CharStopJumping` _currentcharacter))))

(event `InputAxis|MoveForward`
  (params (AxisValue :type "Float (single-precision)"))
  (bind _currentcharacter (`self.CurrentCharacter`))
  ;[1 1 1] Movement binding
  (if (!= AxisValue 0.0)
    (if (`KismetSystemLibrary.IsValid` _currentcharacter)
      (`Pawn.AddMovementInput` _currentcharacter (`self.GetActorForwardVector` _currentcharacter) AxisValue false))))

(event `InputAxis|MoveRight`
  (params (AxisValue :type "Float (single-precision)"))
  (bind _currentcharacter (`self.CurrentCharacter`))
  ;[1 1 1] Movement binding
  (if (!= AxisValue 0.0)
    (if (`KismetSystemLibrary.IsValid` _currentcharacter)
      (`Pawn.AddMovementInput` _currentcharacter (`self.GetActorRightVector` _currentcharacter) AxisValue false))))

(event `self.ReceiveBeginPlay`
  (bind _returnvalue (`|CreateWidget` "/Game/UI/IngameUI.IngameUI_C"))
  (bind _output_get (set `self.CurrentIngameUI` _returnvalue))
  (`UserWidget.AddToViewport` _output_get 0))

(fn `UserConstructionScript`)